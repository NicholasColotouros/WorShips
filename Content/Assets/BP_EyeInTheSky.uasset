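; BP_EyeInTheSky is a temporary overhead targeting pawn for casting a spell from above.
; On possession, a timeline eases the spring arm out toward EyeHeight.
; CastSpell spawns a BP_Ballista at the camera's XY position and a fixed height, with zero projectile velocity.
; Releasing TargetSpell hands possession back to the Character, and the pawn destroys itself when unpossessed.
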(event EventPossessed
  (params (NewController :type Controller%20Object%20Reference))
  (bind _0_to_1 (Timeline|ZoomOut Play)
    (:Update
      (Variables|/Script/Engine.SpringArmComponent|SetTargetArmLength (Variables|Default|GetCameraBoom) (Math|Interpolation|Ease "Linear" _0_to_1 (Variables|/Script/Engine.SpringArmComponent|GetTargetArmLength (Variables|Default|GetCameraBoom)) (Variables|Default|GetEyeHeight))))))

(event EventUnpossessed
  (params (OldController :type Controller%20Object%20Reference))
  ;[1 1 1] Discard and destroy
  (Actor|DestroyActor))

(event Input|ActionEvents|InputActionCastSpell
  (params (Key :type Key%20Structure :default "AnyKey"))
  (bind _cameracomponent (Variables|Default|GetCameraComponent))
  (bind _returnvalue (Transformation|GetWorldLocation _cameracomponent))
  (bind (_x _y) (Math|Vector|BreakVector _returnvalue))
  (:Pressed
    (Game|SpawnActorfromClass "/Game/ShipsAndExamples/Cannonz/BP_Ballista.BP_Ballista_C" (Math|Conversions|ToTransform(Vector) (Math|Vector|MakeVector _x _y 6e+02)) "AlwaysSpawn" 0 0.0 0)))

(event Input|ActionEvents|InputActionTargetSpell
  (params (Key :type Key%20Structure :default "AnyKey"))
  (:Released
    (Pawn|Possess (Game|GetPlayerController 0) (Variables|Default|GetCharacter))))

(fn ConstructionScript)