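; A possessable ballista pawn that players can take over and swivel within yaw limits.
; Capsule overlaps set or clear it as the local ThirdPersonCharacter's InteractionPawn.
; On possession it creates a spring-arm camera at runtime and spawns a ThirdPersonCharacter teleported to the operator spot.
; Turn input sends clamped base rotation through ServerTurn, applied under authority; look-up input is unimplemented and BroadcastTurn is never called.
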(event OnComponentBeginOverlap(Capsule)
  (params (OtherActor :type Actor%20Object%20Reference) (OtherComp :type Primitive%20Component%20Object%20Reference) (OtherBodyIndex :type Integer) (bFromSweep :type Boolean) (SweepResult :type Hit%20Result%20Structure%20%28by%20ref%29))
  (CallFunction|SetPossessionPawn OtherActor true))

(event OnComponentEndOverlap(Capsule)
  (params (OtherActor :type Actor%20Object%20Reference) (OtherComp :type Primitive%20Component%20Object%20Reference) (OtherBodyIndex :type Integer))
  (CallFunction|SetPossessionPawn OtherActor false))

(event Custom|ServerTurn
  (params (Rotation :type Rotator))
  ;[1 1 1] Network Turning
  (Networking|SwitchHasAuthority
    (:Authority
      (Transformation|SetRelativeRotation (Variables|Default|GetBallistaBase) Rotation false false))))

(event Custom|BroadcastTurn
  (params (Rotation :type Rotator))
  ;[1 1 1] Network Turning
  (Transformation|SetRelativeRotation (Variables|Default|GetBallistaBase) Rotation false false))

(event Custom|ClientCreateCamera
  ;[1 1 1] On Possession
  (bind _returnvalue (AddComponent|AddSpringArmComponent true))
  (bind _output_get (Variables|Default|SetSpringArm _returnvalue))
  (Class|SceneComponent|Attachto _returnvalue (Variables|Default|GetSpringArmLoc) "None" "SnapToTarget" true)
  (Variables|/Script/Engine.SpringArmComponent|SetTargetArmLength (Variables|Default|GetSpringArm) 3e+02) ; Default zoom
  (Variables|/Script/Engine.SpringArmComponent|SetbDoCollisionTest (Variables|Default|GetSpringArm) false)
  (bind _returnvalue_2 (AddComponent|AddCameraComponent true))
  (Class|SceneComponent|Attachto _returnvalue_2 (Variables|Default|GetSpringArm) "None" "SnapToTarget" true))

(event Custom|PossessedNetwork
  (params (NewController :type Controller%20Object%20Reference))
  (bind _operatorloc (Variables|Default|GetOperatorLoc))
  ;[1 1 1] On Possession
  (bind _returnvalue (Game|SpawnActorfromClass "/Game/ThirdPersonCPP/Blueprints/ThirdPersonCharacter.ThirdPersonCharacter_C" (Transformation|GetActorTransform NewController) "AlwaysSpawn" 0 0 0))
  (bind _output_get (Variables|Default|SetCurrentlyPossessing _returnvalue))
  (Transformation|Teleport _output_get (Transformation|GetWorldLocation _operatorloc) "0, 0, 0")
  (Class|Actor|AttachRootComponentto _operatorloc "None" "KeepWorldPosition" true))

(event EventTurn
  (params (axisValue :type Float%20%28single-precision%29))
  ;[1 1 1] Network Turning
  (CallFunction|ServerTurn (Math|Rotator|MakeRotator 0.0 0.0 (Math|Float|ClampAngle (+ axisValue (.Yaw (Math|Rotator|BreakRotator (.Rotation (Math|Transform|BreakTransform (Transformation|GetRelativeTransform (Variables|Default|GetBallistaBase))))))) (Variables|Default|GetMinBaseRotation) (Variables|Default|GetMaxBaseRotation)))))

(event EventPossessed
  (params (NewController :type Controller%20Object%20Reference))
  ;[1 1 1] On Possession
  (CallFunction|ClientCreateCamera)
  (CallFunction|PossessedNetwork NewController))

(event Input|AxisEvents|InputAxisTurnRate
  (params (AxisValue :type Float%20%28single-precision%29))
  (Class|WorshipVehicle|Turn (* AxisValue (Variables|Default|GetBaseTurnRate) (Utilities|Time|GetWorldDeltaSeconds))))

(event Input|AxisEvents|InputAxisLookUpRate
  (params (AxisValue :type Float%20%28single-precision%29)))

(fn ConstructionScript)

(fn SetPossessionPawn
  (params (Actor :type Actor%20Object%20Reference) (IsEntering :type Boolean))
  (bind _asthird_person_character (Utilities|Casting|CastToThirdPersonCharacter Actor))
  (Utilities|IsValid (Pawn|GetController _asthird_person_character)
    (:Is%20Valid
      (if (Pawn|IsLocalPlayerController (Pawn|GetController _asthird_person_character))
        ;[1 1 1] If exiting the volume, set ref to null
        (if IsEntering
          (Variables|/Game/ThirdPersonCPP/Blueprints/ThirdPersonCharacter.ThirdPersonCharacter_C|SetInteractionPawn _asthird_person_character self)
          (else
            (Variables|/Game/ThirdPersonCPP/Blueprints/ThirdPersonCharacter.ThirdPersonCharacter_C|SetInteractionPawn _asthird_person_character 0)))))))