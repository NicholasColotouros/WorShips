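; Game mode that serves as the server-side spawner for water abilities, Man O' War actors and player respawns.
; Its spawn events check authority before creating water walls, tidal waves or Man O' Wars.
; Respawn possesses a new ThirdPersonCharacter above the first boat found, or at a fixed fallback point.
; BeginPlay binds player 0's character destruction to show a death widget after a short delay.
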(event Custom|spawnManofwar
  (params (Location :type Transform))
  (Networking|SwitchHasAuthority
    (:Authority
      (Game|SpawnActorfromClass "/Game/ShipsAndExamples/ManOfWar/BP_ManOfWar.BP_ManOfWar_C" Location "AdjustIfPossibleButDontSpawnIfColliding" 0 0))))

(event Custom|MakeRespawnWidget
  (Utilities|FlowControl|Delay 0 0.5)
  (bind _returnvalue (UserInterface|CreateWidget "/Game/UI/Widgets/Widget_Death.Widget_Death_C"))
  (UserInterface|Viewport|AddtoViewport _returnvalue 0)
  (Input|SetInputModeGameandUI 0 _returnvalue false false))

(event Custom|GMSpawnTidalWave
  (params (Player%20Contoller :type Player%20Controller%20Object%20Reference) (Location :type Transform) (Rotation :type Rotator))
  ;[1 1 1] Tidal Wave
  (Utilities|IsValid Player%20Contoller
    (:Is%20Valid
      (Networking|SwitchHasAuthority
        (:Authority
          (Game|SpawnActorfromClass "/Game/Assets/WaterWave.WaterWave_C" Location "AlwaysSpawn" 0 5e+02 Rotation "0.000000,0.000000,0.000000"))))))

(event Custom|Respawn
  (params (PlayerController :type Player%20Controller%20Object%20Reference))
  ;[1 1 1] Respawn
  (bind _outactors (Actor|GetAllActorsOfClass "/Game/Assets/BP_Boat.BP_Boat_C"))
  (Utilities|IsValid PlayerController
    (:Is%20Valid
      (Networking|SwitchHasAuthority
        (:Authority
          (if (Utilities|IsValid (Utilities|Array|Get(acopy) _outactors))
            (bind _returnvalue (Game|SpawnActorfromClass "/Game/ThirdPersonCPP/Blueprints/ThirdPersonCharacter.ThirdPersonCharacter_C" (Math|Transform|MakeTransform (+ (.Location (Math|Transform|BreakTransform (Transformation|GetActorTransform (Utilities|Array|Get(acopy) _outactors)))) "0, 0,300.000000") (.Rotation (Math|Transform|BreakTransform (Transformation|GetActorTransform (Utilities|Array|Get(acopy) _outactors)))) (.Scale (Math|Transform|BreakTransform (Transformation|GetActorTransform (Utilities|Array|Get(acopy) _outactors))))) "Undefined" 0 0 0))
            (Utilities|IsValid _returnvalue
              (:Is%20Valid
                (Pawn|Possess PlayerController _returnvalue)))
            (else
              (bind _returnvalue_2 (Game|SpawnActorfromClass "/Game/ThirdPersonCPP/Blueprints/ThirdPersonCharacter.ThirdPersonCharacter_C" (Math|Transform|MakeTransform "0, 0,1000.000000") "Undefined" 0 0 0))
              (Utilities|IsValid _returnvalue_2
                (:Is%20Valid
                  (Pawn|Possess PlayerController _returnvalue_2))))))))))

(event Custom|GMSpawnWaterWall
  (params (Player%20Contoller :type Player%20Controller%20Object%20Reference) (Location :type Transform) (Rotation :type Rotator))
  ;[1 1 1] Water Wall
  (Utilities|IsValid Player%20Contoller
    (:Is%20Valid
      (Networking|SwitchHasAuthority
        (:Authority
          (Game|SpawnActorfromClass "/Game/Assets/WaterWall.WaterWall_C" Location "AlwaysSpawn" 0 Rotation 0))))))

(event Custom|Wall
  (params (Player%20Controller :type Player%20Controller%20Object%20Reference) (Pawn :type Pawn%20Object%20Reference))
  ;[1 1 1] Water Wall
  (Development|PrintString 0)
  (Utilities|IsValid Player%20Controller
    (:Is%20Valid
      (Networking|SwitchHasAuthority
        (:Authority
          (Game|SpawnActorfromClass "/Game/Assets/WaterWall.WaterWall_C" (Math|Conversions|ToTransform(Vector) (+ (Transformation|GetActorLocation Pawn) (* (Transformation|GetActorForwardVector Pawn) 1e+03))) "AlwaysSpawn" 0 (Transformation|GetActorRotation Pawn) 0))))))

(event EventBeginPlay
  (bind _asthird_person_character (Utilities|Casting|CastToThirdPersonCharacter (Game|GetPlayerCharacter 0)))
  (Game|BindEventtoOnDestroyed _asthird_person_character (delegate Custom|MakeRespawnWidget)))

(fn ConstructionScript)